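; PC_Tank is the tank player controller, handling input setup and the pause menu.
; On possess, it adds the IMC_Tank Enhanced Input mapping context.
; IA_Pause toggles game pause, creating a fresh W_Pause widget with cursor and game-and-UI input focused on it.
; Unpausing removes the widget, restores game-only input and hides the cursor.
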(event `self.ReceivePossess`
  (params (PossessedPawn :type "Pawn Object Reference"))
  (`EnhancedInputSubsystemInterface.AddMappingContext` (subsystem `EnhancedInputLocalPlayerSubsystem`) "/Game/TankProject/Player/Input/IMC_Tank.IMC_Tank" 0 (struct)))

(event `EnhancedInput|/Game/TankProject/Player/Input/IA_Pause`
  (params (ActionValue :type Boolean) (ElapsedSeconds :type "Float (double-precision)") (TriggeredSeconds :type "Float (double-precision)") (InputAction :type "InputAction Object Reference" :default "/Game/TankProject/Player/Input/IA_Pause.IA_Pause"))
  (:`Started`
    (if (not (`GameplayStatics.IsGamePaused`))
      (`GameplayStatics.SetGamePaused` true)
      (bind _returnvalue (`|CreateWidget` "/Game/TankProject/UI/W_Pause.W_Pause_C"))
      (bind _output_get (set `self.PauseUI` _returnvalue))
      (`UserWidget.AddToViewport` _output_get 0)
      (set `self.bShowMouseCursor` true)
      (`WidgetBlueprintLibrary.SetInputMode_GameAndUIEx` self (`self.PauseUI`))
      (else
        (`Widget.RemoveFromParent` (`self.PauseUI`))
        (`WidgetBlueprintLibrary.SetInputMode_GameOnly` self)
        (set `self.bShowMouseCursor` false)
        (`GameplayStatics.SetGamePaused` false)))))

(fn `UserConstructionScript`)