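; BP_Camera is a follow camera that becomes player 0's view target and tracks the pawns in PlayerPawns.
; BeginPlay or Init refills that array, currently with only player 0's pawn.
; Each tick lerps the Sphere toward the pawns' average location by MovementSpeed.
; It also zooms by interpolating spring arm length toward the largest pairwise pawn distance, clamped between minimum and maximum lengths.
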(event `self.ReceiveBeginPlay`
  (`KismetArrayLibrary.Array_Clear` (`self.playerPawns`) :!label _label)
  (`KismetArrayLibrary.Array_Add` (`self.playerPawns`) (`GameplayStatics.GetPlayerPawn` 0))
  (`PlayerController.SetViewTargetWithBlend` (`GameplayStatics.GetPlayerController` 0) self 0.0 "VTBlend_Linear" 0.0 false))

(event `Init`
  (goto _label))

(event `self.ReceiveTick`
  (params (DeltaSeconds :type "Float (single-precision)"))
  ;[1 1 1] Move Camera on Tick
  (`self.CalculateCameraMovement`)
  (`self.CalculateCameraDistance`))

(fn `CalculateCameraDistance`
  (bind _pawn (`self.pawn`))
  (for (_array_element _array_index) (`self.playerPawns`)
    (set `self.pawn` _array_element)
    (for _index (range (+ _array_index 1) (`KismetArrayLibrary.Array_Length` (`self.playerPawns`)))
      (bind _output (`|GetArrayItem` (`self.playerPawns`) _index))
      (if (and (`KismetSystemLibrary.IsValid` _pawn) (`KismetSystemLibrary.IsValid` _output))
        (`KismetArrayLibrary.Array_Add` (`self.distance`) (`self.GetDistanceTo` _pawn _output)))))
  (set `SpringArmComponent.TargetArmLength` (`KismetMathLibrary.FInterpTo` (`SpringArmComponent.TargetArmLength` (`self.SpringArm`)) (`KismetMathLibrary.FClamp` (`.MaxValue` (`KismetMathLibrary.MaxOfFloatArray` (`self.distance`))) (`self.minArmLength`) (`self.maxArmLength`)) (`GameplayStatics.GetWorldDeltaSeconds`) 3.0) (`self.SpringArm`))
  (`KismetArrayLibrary.Array_Clear` (`self.distance`)))

(fn `CalculateCameraMovement`
  (set `self.previousLocation` (`SceneComponent.K2_GetComponentLocation` (`self.Sphere`)))
  (bind _returnvalue (`GameplayStatics.GetActorArrayAverageLocation` (`self.playerPawns`)))
  (`SceneComponent.K2_SetWorldLocation` (`self.Sphere`) (`KismetMathLibrary.VLerp` (`self.previousLocation`) _returnvalue (`self.movementSpeed`)) false false))

(fn `UserConstructionScript`)