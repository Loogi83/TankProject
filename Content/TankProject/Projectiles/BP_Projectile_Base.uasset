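; BP_Projectile_Base is the base projectile Blueprint in TankProject, handling impacts and a limited bounce count.
; On a blocking hit, it sends HitMessage to actors implementing BPI_Hit and destroys itself.
; Other blocking hits call Bounce, which only increments a counter and destroys the projectile once MaxBounceCount is reached.
; When hit by another bullet, it prints a debug message and destroys itself.
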(event `self.ReceiveHit`
  (params (MyComp :type "PrimitiveComponent Object Reference") (Other :type "Actor Object Reference") (OtherComp :type "PrimitiveComponent Object Reference") (bSelfMoved :type Boolean) (HitLocation :type "Vector Structure") (HitNormal :type "Vector Structure") (NormalImpulse :type "Vector Structure") (Hit :type "HitResult Structure (by ref)"))
  (bind (_bblockinghit _binitialoverlap _time _distance _location _impactpoint _normal _impactnormal _physmat _hitactor) (`GameplayStatics.BreakHitResult` Hit))
  (if _bblockinghit
    (if (`KismetSystemLibrary.DoesImplementInterface` _hitactor "/Game/TankProject/Projectiles/BPI_Hit.BPI_Hit_C")
      (message `/Game/TankProject/Projectiles/BPI_Hit.Hit` _hitactor self)
      (`self.K2_DestroyActor`)
      (else
        (`self.Bounce`)))))

(event `/Game/TankProject/Projectiles/BPI_Hit.Hit`
  (params (Bullet :type "/Game/TankProject/Projectiles/BP_Projectile_Base Object Reference"))
  (`KismetSystemLibrary.PrintString` (`KismetStringLibrary.Concat_StrStr` (`KismetSystemLibrary.GetDisplayName` self) " was hit by " (`KismetSystemLibrary.GetDisplayName` Bullet)))
  (`self.K2_DestroyActor`))

(fn `Bounce`
  (if (>= (`self.BounceCount`) (`self.MaxBounceCount`))
    (`self.K2_DestroyActor`)
    (else
      (`/Engine/EditorBlueprintResources/StandardMacros.IncrementInt` (`self.BounceCount`)))))

(fn `UserConstructionScript`)