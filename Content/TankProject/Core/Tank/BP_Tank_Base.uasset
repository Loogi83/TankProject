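; Base player-controlled tank with stick-driven movement, independent turret aim, projectile fire and capped mine deployment.
; The body turns at constant speed toward the input, or its reverse if closer, and moves only once aligned.
; A hit reports the kill, plays explosion effects, leaves a fading decal, then hides and sinks the tank instead of destroying it.
; RespawnTank restores input, hit detection and audio; game end disables input.
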(event `Init`
  (params (GameMode :type "/Game/TankProject/Core/GameModes/GM_Tank Object Reference"))
  (add `/Game/TankProject/Core/GameModes/GM_Tank.OnGameEnd` GameMode (`|CreateDelegate` :!event `OnGameEnd`)))

(event `self.ReceiveTick`
  (params (DeltaSeconds :type "Float (single-precision)"))
  (`KismetSystemLibrary.DrawDebugString` (0.0 0.0 0.0) (`KismetTextLibrary.Conv_TextToString` (`|FormatText` "{Controller} {Number}" (`self.GetController`) (`self.TankID`))) self (struct :`R` 0.608366 :`B` 1.0 :`A` 1.0)))

(event `EnhancedInput|/Game/TankProject/Player/Input/IA_Aim`
  (params (ActionValue :type "Vector2D Structure") (ElapsedSeconds :type "Float (double-precision)") (TriggeredSeconds :type "Float (double-precision)") (InputAction :type "InputAction Object Reference" :default "/Game/TankProject/Player/Input/IA_Aim.IA_Aim"))
  ;[0.7854 1 0] Aim Turret
  (:`Triggered`
    (if (`self.CanReceiveInput`)
      (set `self.AimRotation` (`KismetMathLibrary.MakeRotator` 0.0 0.0 (`KismetMathLibrary.DegAtan2` ActionValue_Y ActionValue_X)))
      (`self.RotateTurret`))))

(event `EnhancedInput|/Game/TankProject/Player/Input/IA_Movement`
  (params (ActionValue :type "Vector2D Structure") (ElapsedSeconds :type "Float (double-precision)") (TriggeredSeconds :type "Float (double-precision)") (InputAction :type "InputAction Object Reference" :default "/Game/TankProject/Player/Input/IA_Movement.IA_Movement"))
  (bind _tankaudio (`self.TankAudio`))
  (bind _canreceiveinput (`self.CanReceiveInput`))
  ;[0 0.2089 1] Movement
  (:`Triggered`
    (if _canreceiveinput
      (set `self.MovementRotation` (`KismetMathLibrary.MakeRotator` 0.0 0.0 (`KismetMathLibrary.DegAtan2` ActionValue_Y ActionValue_X)))
      (`self.Get Movement Direction`)
      (bind _canmoveforward (`self.RotateBody`))
      (if _canmoveforward
        (`self.K2_AddActorWorldOffset` (* (`KismetMathLibrary.Conv_RotatorToVector` (`self.MovementRotation`)) (* (`self.ForwardSpeed`) (`GameplayStatics.GetWorldDeltaSeconds`))) true))))
  (:`Started`
    (if _canreceiveinput
      (`AudioParameterControllerInterface.SetTriggerParameter` _tankaudio "MoveStart")))
  (:`Completed`
    (`AudioParameterControllerInterface.SetTriggerParameter` _tankaudio "MoveStop")))

(event `EnhancedInput|/Game/TankProject/Player/Input/IA_Mine`
  (params (ActionValue :type Boolean) (ElapsedSeconds :type "Float (double-precision)") (TriggeredSeconds :type "Float (double-precision)") (InputAction :type "InputAction Object Reference" :default "/Game/TankProject/Player/Input/IA_Mine.IA_Mine"))
  (bind (_returnvalue_x _returnvalue_y) (`KismetMathLibrary.BreakVector` (`self.K2_GetActorLocation`)))
  ;[0 1 0.4799] Deploy Mine
  (:`Started`
    (if (`self.CanReceiveInput`)
      (if (< (`self.CurrentMines`) (`self.MaxMines`))
        (bind _returnvalue (`|SpawnActorFromClass` (`self.DefaultMine`) (`KismetMathLibrary.MakeTransform` (`KismetMathLibrary.MakeVector` _returnvalue_x _returnvalue_y)) "AlwaysSpawn" "MultiplyWithRoot" null 500.0 10.0 self))
        (`/Game/TankProject/Core/Weapons/Secondary/BP_Mine_Base.Init` _returnvalue)
        (`/Engine/EditorBlueprintResources/StandardMacros.IncrementInt` (`self.CurrentMines`))))))

(event `EnhancedInput|/Game/TankProject/Player/Input/IA_Fire`
  (params (ActionValue :type Boolean) (ElapsedSeconds :type "Float (double-precision)") (TriggeredSeconds :type "Float (double-precision)") (InputAction :type "InputAction Object Reference" :default "/Game/TankProject/Player/Input/IA_Fire.IA_Fire"))
  (bind (_returnvalue_location _returnvalue_rotation) (`KismetMathLibrary.BreakTransform` (`SceneComponent.GetSocketTransform` (`self.SkeletalMesh`) "FirePoint" "RTS_World")))
  ;[1 0 0] Fire
  (:`Started`
    (if (`self.CanReceiveInput`)
      (`|SpawnActorFromClass` (`self.DefaultProjectile`) (`KismetMathLibrary.MakeTransform` _returnvalue_location _returnvalue_rotation) "AdjustIfPossibleButAlwaysSpawn" "MultiplyWithRoot" null self)
      (`AudioParameterControllerInterface.SetTriggerParameter` (`self.TankAudio`) "Fire"))))

(event `OnGameEnd`
  (params (WinningPlayer :type Integer))
  (set `self.CanReceiveInput` false)
  (`AudioParameterControllerInterface.SetTriggerParameter` (`self.TankAudio`) "MoveStop"))

(event `/Game/TankProject/Core/Weapons/BPI_Hit.Hit`
  (params (Attacker :type "Controller Object Reference"))
  (bind _returnvalue (`self.K2_GetActorLocation`))
  ;[1 0 0] Hit
  (if (`self.CanReceiveHit`)
    (set `self.CanReceiveHit` false)
    (`AudioComponent.SetPaused` (`self.TankAudio`) true)
    (`GameplayStatics.PlaySoundAtLocation` "/Game/TankProject/Core/Tank/Sounds/SW_TankExplode.SW_TankExplode" (`self.K2_GetActorLocation`) (struct) 1.0 1.0 0.0 null null null null)
    (`self.TankDestroyed` (`self.GetController`) Attacker)
    (`NiagaraFunctionLibrary.SpawnSystemAtLocation` "/Game/TankProject/Core/FX/NS_Explosion.NS_Explosion" (`self.K2_GetActorLocation`) (struct) (`KismetMathLibrary.Conv_DoubleToVector` (`self.ExplosionScale`)))
    (`GameplayStatics.PlayWorldCameraShake` "/Game/TankProject/Core/FX/CS_Explosion.CS_Explosion_C" (`PlayerCameraManager.GetCameraLocation` (`GameplayStatics.GetPlayerCameraManager` 0)) 0.0 10.0 1.0 true)
    (`self.SetActorHiddenInGame` true)
    (set `self.CanReceiveInput` false)
    (bind _outhit (`KismetSystemLibrary.LineTraceSingle` _returnvalue (- _returnvalue (* (`self.GetActorUpVector`) 100.0)) "TraceTypeQuery1"))
    (`|ExecutionSequence`
      (:`then_0`
        (bind _returnvalue_2 (`GameplayStatics.SpawnDecalAtLocation` "/Game/TankProject/Core/Tank/M_Cross.M_Cross" (10.0 100.0 100.0) (`.Location` (`GameplayStatics.BreakHitResult` _outhit))))
        (`DecalComponent.SetFadeOut` _returnvalue_2 30.0 1.0 true))
      (:`then_1`
        (`self.K2_SetActorLocation` (0.0 0.0 -100.0) false true)))))

(fn `Get Movement Direction`
  (returns (MovementDirection :type "/Game/TankProject/Core/Tank/EMovementDirection Enum"))
  (bind (_returnvalue_roll _returnvalue_pitch _returnvalue_yaw) (`KismetMathLibrary.BreakRotator` (`KismetMathLibrary.NormalizedDeltaRotator` (`KismetMathLibrary.Conv_VectorToRotator` (`self.GetActorForwardVector`)) (`self.MovementRotation`))))
  (bind _output_get (set `self.MovementDirection` (select `bool` (`KismetMathLibrary.InRange_FloatFloat` _returnvalue_yaw -90.0 90.0) :`false` "NewEnumerator1" :`true` "NewEnumerator0" :!type "/Game/TankProject/Core/Tank/EMovementDirection Enum")))
  (return _output_get))

(fn `RespawnTank`
  (set `self.CanReceiveHit` true)
  (set `self.CanReceiveInput` true)
  (`AudioComponent.SetPaused` (`self.TankAudio`) false))

(fn `RotateBody`
  (returns (CanMoveForward :type Boolean))
  (bind (_movementrotation_roll _movementrotation_pitch _movementrotation_yaw) (`KismetMathLibrary.BreakRotator` (`self.MovementRotation`)))
  (bind (_movementrotation_roll_2 _movementrotation_pitch_2 _movementrotation_yaw_2) (`KismetMathLibrary.BreakRotator` (`self.MovementRotation`)))
  (if (not (== (`self.BodyRotation`) (select `/Game/TankProject/Core/Tank/EMovementDirection` (`self.MovementDirection`) :`NewEnumerator0` (`self.MovementRotation`) :`NewEnumerator1` (`KismetMathLibrary.MakeRotator` _movementrotation_roll _movementrotation_pitch (+ _movementrotation_yaw 180.0))) :`ErrorTolerance` 1.0))
    (bind _output_get (set `self.BodyRotation` (`KismetMathLibrary.RInterpTo_Constant` (`self.BodyRotation`) (select `/Game/TankProject/Core/Tank/EMovementDirection` (`self.MovementDirection`) :`NewEnumerator0` (`self.MovementRotation`) :`NewEnumerator1` (`KismetMathLibrary.MakeRotator` _movementrotation_roll_2 _movementrotation_pitch_2 (+ _movementrotation_yaw_2 180.0))) (`GameplayStatics.GetWorldDeltaSeconds`) (`self.BodyRotateSpeed`))))
    (`self.K2_SetActorRotation` _output_get)
    (bind _output_get_2 (set `self.CanMoveForward` false))
    (return _output_get_2)
    (else
      (bind _output_get_3 (set `self.CanMoveForward` true))
      (return _output_get_3))))

(fn `RotateTurret`
  (set `self.TurretRotation` (`KismetMathLibrary.RInterpTo_Constant` (`self.TurretRotation`) (`self.AimRotation`) (`GameplayStatics.GetWorldDeltaSeconds`) (`self.TurretTurnSpeed`))))

(fn `UserConstructionScript`)