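; Game mode for a local multiplayer tank match that runs setup, scoring, respawning and game end.
; On BeginPlay it recreates local players from the game instance, spawns a tank per spawn point, possesses those with controllers, and builds a shared camera and HUD.
; Tank deaths leave the camera; kills add to the score component, which either ends the match with a results widget or lets the victim respawn.
; Self-kills respawn without scoring.
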(event `self.ReceiveBeginPlay`
  (bind _astank_game_instance (cast `/Game/TankProject/Core/TankGameInstance` (`GameplayStatics.GetGameInstance`)))
  (set `self.As Tank Game Instance` _astank_game_instance)
  (`self.RemovePlayers`)
  (`self.SetUpPlayers` (`KismetMathLibrary.Or_IntInt` (`/Game/TankProject/Core/TankGameInstance.NumberOfPlayers` (`self.As Tank Game Instance`)) 1))
  (bind _outactors (`GameplayStatics.GetAllActorsOfClass` "/Game/TankProject/Core/BP_SpawnPoint.BP_SpawnPoint_C"))
  (set `self.SpawnPoints` _outactors)
  (bind _returnvalue (`|SpawnActorFromClass` "/Game/TankProject/Core/BP_Camera.BP_Camera_C" (`KismetMathLibrary.MakeTransform` (0.0 0.0 0.0)) "Undefined" "MultiplyWithRoot" null null))
  (set `self.CameraActor` _returnvalue)
  (bind _returnvalue_2 (`|CreateWidget` "/Game/TankProject/UI/W_GameHUD.W_GameHUD_C"))
  (set `self.GameHUD` _returnvalue_2)
  (for (_ _array_index) (`self.SpawnPoints`)
    (`self.SpawnTank` _array_index))
  (`/Game/TankProject/Core/BP_Camera.Init` (`self.CameraActor`))
  (`UserWidget.AddToViewport` (`self.GameHUD`) 0)
  (for _array_element (`self.PlayerList`)
    (set `/Game/TankProject/Core/Tank/BP_Tank_Base.CanReceiveInput` true _array_element)))

(event `TankDestroyed`
  (params (PlayerKilled :type "Controller Object Reference") (KilledBy :type "Controller Object Reference"))
  (bind _returnvalue (`Controller.K2_GetPawn` KilledBy))
  (bind _returnvalue_2 (`Controller.K2_GetPawn` PlayerKilled))
  ;[1 1 1] Tank Destroyed
  (`/Game/TankProject/Core/BP_Camera.RemovePlayer` (`self.CameraActor`) _returnvalue_2)
  (if (!= _returnvalue _returnvalue_2)
    (bind (_canend _scoringplayerid) (`/Game/TankProject/Core/AC_PlayerScores.AddScore` (`self.AC_PlayerScores`) (`/Game/TankProject/Core/Tank/BP_Tank_Base.TankID` (cast `/Game/TankProject/Core/Tank/BP_Tank_Base` _returnvalue :!pure true)) 1))
    (if _canend
      (`self.GameEnd` _scoringplayerid)
      (else
        (`/Game/TankProject/Core/BP_SpawnPoint.RespawnTank` (`|GetArrayItem` (`self.SpawnPoints`) (`KismetArrayLibrary.Array_Find` (`self.PlayerList`) (cast `/Game/TankProject/Core/Tank/BP_Tank_Base` _returnvalue_2 :!pure true))) _returnvalue_2 :!label _label)))
    (else
      (goto _label))))

(event `GameEnd`
  (params (WinningPlayer :type Integer))
  (bind _returnvalue (`GameplayStatics.GetPlayerController` 0))
  (`self.OnGameEnd` WinningPlayer)
  (bind _returnvalue_2 (`|CreateWidget` "/Game/TankProject/UI/W_GameEnd.W_GameEnd_C"))
  (`/Game/TankProject/UI/W_GameEnd.SetStats` _returnvalue_2 WinningPlayer (`.Score` (`/Game/TankProject/Core/AC_PlayerScores.GetPlayerScore` (`self.AC_PlayerScores`) WinningPlayer)))
  (`UserWidget.AddToViewport` _returnvalue_2 0)
  (`WidgetBlueprintLibrary.SetInputMode_UIOnlyEx` _returnvalue _returnvalue_2)
  (set `PlayerController.bShowMouseCursor` true _returnvalue))

(fn `RemovePlayers`
  (for _index (range (`GameplayStatics.GetNumLocalPlayerControllers`))
    (`GameplayStatics.RemovePlayer` (`GameplayStatics.GetPlayerControllerFromID` _index) true))
  (return))

(fn `SetUpPlayers`
  (params (NumberOfPlayers :type Integer :default 1))
  (bind _returnvalue (`GameplayStatics.GetPlayerController` 0))
  (for _index (range NumberOfPlayers)
    (bind _returnvalue_2 (`GameplayStatics.CreatePlayer` _index))
    (`KismetArrayLibrary.Array_AddUnique` (`self.PlayerControllerList`) _returnvalue_2))
  (set `PlayerController.bShowMouseCursor` false _returnvalue)
  (`WidgetBlueprintLibrary.SetInputMode_GameOnly` _returnvalue)
  (`WidgetBlueprintLibrary.SetFocusToGameViewport`)
  (return))

(fn `SpawnTank`
  (params (TankID :type Integer))
  (bind _returnvalue (`GameplayStatics.GetPlayerController` TankID))
  (bind _returnvalue_2 (`|SpawnActorFromClass` "/Game/TankProject/Core/Tank/BP_Tank_Base.BP_Tank_Base_C" (`self.GetTransform` (`|GetArrayItem` (`self.SpawnPoints`) TankID)) "AdjustIfPossibleButAlwaysSpawn" "MultiplyWithRoot" null TankID null))
  (`KismetArrayLibrary.Array_AddUnique` (`self.PlayerList`) _returnvalue_2)
  (`/Game/TankProject/Core/BP_Camera.AddPlayer` (`self.CameraActor`) _returnvalue_2)
  (add `/Game/TankProject/Core/Tank/BP_Tank_Base.TankDestroyed` _returnvalue_2 (`|CreateDelegate` :!event `TankDestroyed`))
  (`/Game/TankProject/Core/Tank/BP_Tank_Base.Init` _returnvalue_2 self)
  (`/Engine/EditorBlueprintResources/StandardMacros.IsValid` _returnvalue
    (:`Is Valid`
      (`Controller.Possess` _returnvalue _returnvalue_2)
      (return))
    (:`Is Not Valid`
      (return))))

(fn `UserConstructionScript`)