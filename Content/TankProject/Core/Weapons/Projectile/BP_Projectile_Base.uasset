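; Base projectile Blueprint for a tank project's weapons that limits bounces and notifies the actors it hits.
; On a blocking hit, actors implementing BPI_Hit receive HitMessage with the instigator's controller and the projectile is destroyed.
; Other blocking hits call Bounce, which counts and plays a sound until MaxBounceCount triggers destruction.
; A second hit event destroys it directly, and Destroy plays a sound before removing the actor.
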(event `self.ReceiveHit`
  (params (MyComp :type "PrimitiveComponent Object Reference") (Other :type "Actor Object Reference") (OtherComp :type "PrimitiveComponent Object Reference") (bSelfMoved :type Boolean) (HitLocation :type "Vector Structure") (HitNormal :type "Vector Structure") (NormalImpulse :type "Vector Structure") (Hit :type "HitResult Structure (by ref)"))
  (bind (_bblockinghit _binitialoverlap _time _distance _location _impactpoint _normal _impactnormal _physmat _hitactor) (`GameplayStatics.BreakHitResult` Hit))
  (if _bblockinghit
    (if (`KismetSystemLibrary.DoesImplementInterface` _hitactor "/Game/TankProject/Core/Weapons/BPI_Hit.BPI_Hit_C")
      (message `/Game/TankProject/Core/Weapons/BPI_Hit.Hit` _hitactor (`self.GetInstigatorController` self))
      (`self.Destroy`)
      (else
        (`self.Bounce`)))))

(event `/Game/TankProject/Core/Weapons/BPI_Hit.Hit`
  (params (Attacker :type "Controller Object Reference"))
  (`self.Destroy`))

(fn `Bounce`
  (if (>= (`self.BounceCount`) (`self.MaxBounceCount`))
    (`self.Destroy`)
    (else
      (`/Engine/EditorBlueprintResources/StandardMacros.IncrementInt` (`self.BounceCount`)
        (:`  `
          (`GameplayStatics.PlaySoundAtLocation` "/Game/TankProject/Core/Weapons/Sounds/A_Bounce_Cue.A_Bounce_Cue" (`self.K2_GetActorLocation`) (struct) 1.0 1.0 0.0 null null null null))))))

(fn `Destroy`
  (`GameplayStatics.PlaySoundAtLocation` "/Game/TankProject/Core/Weapons/Sounds/A_BulletDestroy_Cue.A_BulletDestroy_Cue" (`self.K2_GetActorLocation`) (struct) 1.0 1.0 0.0 null null null null)
  (`self.K2_DestroyActor`))

(fn `UserConstructionScript`)