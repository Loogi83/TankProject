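; Tank spawn point that brings a tank back into play at its own transform after a delay.
; A box tracks overlapping actors, and when the respawn timer fires each one receives a hit message credited to the respawning tank's controller.
; The tank is then teleported in, unhidden, re-added to the game mode's camera actor, and allowed to receive hits and input again.
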(event `self.ReceiveBeginPlay`
  ;[1 1 1] Begin Play
  (bind _asgm_tank (cast `/Game/TankProject/Core/GameModes/GM_Tank` (`GameplayStatics.GetGameMode`)))
  (set `self.As GM Tank` _asgm_tank))

(event `RespawnTank`
  (params (TankToRespawn :type "Pawn Object Reference"))
  ;[1 1 1] Respawn Tank
  (set `self.Tank to Respawn` TankToRespawn)
  (bind _returnvalue (`KismetSystemLibrary.K2_SetTimerDelegate` (delegate `Respawn`) (`self.RespawnDelay`)))
  (set `self.RespawnHandle` _returnvalue))

(event `Respawn`
  (bind _tank_to_respawn (`self.Tank to Respawn`))
  (bind _asbp_tank_base (cast `/Game/TankProject/Core/Tank/BP_Tank_Base` _tank_to_respawn :!pure true))
  ;[1 1 1] Respawn Tank
  (for _array_element (`self.OverlappingActors`)
    (message `/Game/TankProject/Core/Weapons/BPI_Hit.Hit` _array_element (`Pawn.GetController` (`self.Tank to Respawn`))))
  (`self.K2_SetActorTransform` (`self.Tank to Respawn`) (`self.GetTransform`) false true)
  (`self.SetActorHiddenInGame` _tank_to_respawn false)
  (`/Game/TankProject/Core/BP_Camera.AddPlayer` (`/Game/TankProject/Core/GameModes/GM_Tank.CameraActor` (`self.As GM Tank`)) _tank_to_respawn)
  (set `/Game/TankProject/Core/Tank/BP_Tank_Base.CanReceiveHit` true _asbp_tank_base)
  (set `/Game/TankProject/Core/Tank/BP_Tank_Base.CanReceiveInput` true _asbp_tank_base)
  (set `self.Tank to Respawn` null))

(event `self.Box.OnComponentBeginOverlap`
  (params (OverlappedComponent :type "PrimitiveComponent Object Reference") (OtherActor :type "Actor Object Reference") (OtherComp :type "PrimitiveComponent Object Reference") (OtherBodyIndex :type Integer) (bFromSweep :type Boolean) (SweepResult :type "HitResult Structure (by ref)"))
  ;[1 1 1] Overlapping Spawn Point
  (`KismetArrayLibrary.Array_AddUnique` (`self.OverlappingActors`) OtherActor))

(event `self.Box.OnComponentEndOverlap`
  (params (OverlappedComponent :type "PrimitiveComponent Object Reference") (OtherActor :type "Actor Object Reference") (OtherComp :type "PrimitiveComponent Object Reference") (OtherBodyIndex :type Integer))
  ;[1 1 1] Overlapping Spawn Point
  (if (`KismetArrayLibrary.Array_Contains` (`self.OverlappingActors`) OtherActor)
    (`KismetArrayLibrary.Array_RemoveItem` (`self.OverlappingActors`) OtherActor)))

(fn `UserConstructionScript`)