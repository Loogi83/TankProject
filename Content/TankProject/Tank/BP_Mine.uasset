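; BP_Mine is a tank-game mine that explodes and damages nearby objects through the BPI_Hit interface.
; It arms once its instigator leaves the capsule, after which any valid overlap triggers it; Init also starts a fuse timer.
; Overlaps and Hit events feed a once-only Explode, which sphere-traces with debug drawing, sends HitMessage with the instigator's controller, then destroys the mine.
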(event `self.Capsule.OnComponentEndOverlap`
  (params (OverlappedComponent :type "PrimitiveComponent Object Reference") (OtherActor :type "Actor Object Reference") (OtherComp :type "PrimitiveComponent Object Reference") (OtherBodyIndex :type Integer))
  ;[1 1 1] On Spawn
  (if (== OtherActor (`self.GetInstigator`))
    (`/Engine/EditorBlueprintResources/StandardMacros.DoOnce` false
      (:`Completed`
        (set `self.CanExplode` true)))))

(event `Init`
  ;[1 1 1] Start Timer
  (`KismetSystemLibrary.K2_SetTimerDelegate` (`|CreateDelegate` :!event `Explode`) (`self.FuseTime`)))

(event `self.Capsule.OnComponentBeginOverlap`
  (params (OverlappedComponent :type "PrimitiveComponent Object Reference") (OtherActor :type "Actor Object Reference") (OtherComp :type "PrimitiveComponent Object Reference") (OtherBodyIndex :type Integer) (bFromSweep :type Boolean) (SweepResult :type "HitResult Structure (by ref)"))
  ;[1 1 1] On Overlap
  (if (`self.CanExplode`)
    (`/Engine/EditorBlueprintResources/StandardMacros.IsValid` OtherActor
      (:`Is Valid`
        (`self.Explode`)))))

(event `Explode`
  (bind _returnvalue (`self.K2_GetActorLocation`))
  ;[1 0.008761 0] Explode
  (`/Engine/EditorBlueprintResources/StandardMacros.DoOnce` false
    (:`Completed`
      (bind (_outhits _returnvalue_2) (`KismetSystemLibrary.SphereTraceMultiForObjects` :`Start` _returnvalue :`End` _returnvalue :`Radius` (`self.Radius`) :`ObjectTypes` (`|MakeArray` "ObjectTypeQuery3" "ObjectTypeQuery7" :!type "EObjectTypeQuery Enum") :`DrawDebugType` "ForDuration"))
      (if _returnvalue_2
        (for _array_element _outhits
          (bind (_bblockinghit _binitialoverlap _time _distance _location _impactpoint _normal _impactnormal _physmat _hitactor) (`GameplayStatics.BreakHitResult` _array_element))
          (if (`KismetSystemLibrary.DoesImplementInterface` _hitactor "/Game/TankProject/Projectiles/BPI_Hit.BPI_Hit_C")
            (message `/Game/TankProject/Projectiles/BPI_Hit.Hit` _hitactor (`self.GetInstigatorController`)))))
      (`self.K2_DestroyActor`))))

(event `/Game/TankProject/Projectiles/BPI_Hit.Hit`
  (params (Attacker :type "Controller Object Reference"))
  (`self.Explode`))

(fn `UserConstructionScript`)