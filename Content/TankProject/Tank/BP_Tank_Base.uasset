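; Base player-controlled tank that drives, aims and fires through Enhanced Input actions.
; Move input becomes a world yaw; the body turns at constant speed toward it, forward or reversed, whichever is closer, and translates without sweep only once aligned.
; Aim input separately interpolates a TurretRotation variable, without applying it to a component here.
; Fire spawns BP_Projectile_Base at the mesh's FirePoint socket.
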(event `EnhancedInput|/Game/TankProject/Player/Input/IA_Aim`
  (params (ActionValue :type "Vector2D Structure") (ElapsedSeconds :type "Float (double-precision)") (TriggeredSeconds :type "Float (double-precision)") (InputAction :type "InputAction Object Reference" :default "/Game/TankProject/Player/Input/IA_Aim.IA_Aim"))
  ;[0.7854 1 0] Aim Turret
  (:`Triggered`
    (set `self.AimRotation` (`KismetMathLibrary.MakeRotator` 0.0 0.0 (`KismetMathLibrary.DegAtan2` ActionValue_Y ActionValue_X)))
    (`self.RotateTurret`)))

(event `EnhancedInput|/Game/TankProject/Player/Input/IA_Movement`
  (params (ActionValue :type "Vector2D Structure") (ElapsedSeconds :type "Float (double-precision)") (TriggeredSeconds :type "Float (double-precision)") (InputAction :type "InputAction Object Reference" :default "/Game/TankProject/Player/Input/IA_Movement.IA_Movement"))
  ;[0 0.2089 1] Movement
  (:`Triggered`
    (bind _output_get (set `self.MovementRotation` (`KismetMathLibrary.MakeRotator` 0.0 0.0 (`KismetMathLibrary.DegAtan2` ActionValue_Y ActionValue_X))))
    (`SceneComponent.K2_SetWorldRotation` (`self.MovementInput`) _output_get false false)
    (`self.Get Movement Direction`)
    (bind _canmove (`self.RotateBody`))
    (if _canmove
      (`self.K2_AddActorWorldOffset` (* (`KismetMathLibrary.Conv_RotatorToVector` (`self.MovementRotation`)) (`self.ForwardSpeed`))))))

(event `EnhancedInput|/Game/TankProject/Player/Input/IA_Fire`
  (params (ActionValue :type Boolean) (ElapsedSeconds :type "Float (double-precision)") (TriggeredSeconds :type "Float (double-precision)") (InputAction :type "InputAction Object Reference" :default "/Game/TankProject/Player/Input/IA_Fire.IA_Fire"))
  (bind (_returnvalue_location _returnvalue_rotation) (`KismetMathLibrary.BreakTransform` (`SceneComponent.GetSocketTransform` (`self.SkeletalMesh`) "FirePoint" "RTS_World")))
  (:`Started`
    (`|SpawnActorFromClass` "/Game/TankProject/Projectiles/BP_Projectile_Base.BP_Projectile_Base_C" (`KismetMathLibrary.MakeTransform` _returnvalue_location _returnvalue_rotation) "AdjustIfPossibleButAlwaysSpawn" "MultiplyWithRoot" null self)))

(fn `Get Movement Direction`
  (returns (MovementDirection :type "/Game/TankProject/Tank/EMovementDirection Enum"))
  (bind (_returnvalue_roll _returnvalue_pitch _returnvalue_yaw) (`KismetMathLibrary.BreakRotator` (`KismetMathLibrary.NormalizedDeltaRotator` (`KismetMathLibrary.Conv_VectorToRotator` (`self.GetActorForwardVector`)) (`self.MovementRotation`))))
  (bind _output_get (set `self.MovementDirection` (select `bool` (`KismetMathLibrary.InRange_FloatFloat` _returnvalue_yaw -90.0 90.0) :`false` "NewEnumerator1" :`true` "NewEnumerator0" :!type "/Game/TankProject/Tank/EMovementDirection Enum")))
  (return _output_get))

(fn `RotateBody`
  (returns (CanMove :type Boolean))
  (bind (_movementrotation_roll _movementrotation_pitch _movementrotation_yaw) (`KismetMathLibrary.BreakRotator` (`self.MovementRotation`)))
  (bind (_movementrotation_roll_2 _movementrotation_pitch_2 _movementrotation_yaw_2) (`KismetMathLibrary.BreakRotator` (`self.MovementRotation`)))
  (if (not (== (`self.BodyRotation`) (select `/Game/TankProject/Tank/EMovementDirection` (`self.MovementDirection`) :`NewEnumerator0` (`self.MovementRotation`) :`NewEnumerator1` (`KismetMathLibrary.MakeRotator` _movementrotation_roll _movementrotation_pitch (+ _movementrotation_yaw 180.0))) :`ErrorTolerance` 1.0))
    (bind _output_get (set `self.BodyRotation` (`KismetMathLibrary.RInterpTo_Constant` (`self.BodyRotation`) (select `/Game/TankProject/Tank/EMovementDirection` (`self.MovementDirection`) :`NewEnumerator0` (`self.MovementRotation`) :`NewEnumerator1` (`KismetMathLibrary.MakeRotator` _movementrotation_roll_2 _movementrotation_pitch_2 (+ _movementrotation_yaw_2 180.0))) (`GameplayStatics.GetWorldDeltaSeconds`) (`self.BodyRotateSpeed`))))
    (`self.K2_SetActorRotation` _output_get)
    (bind _output_get_2 (set `self.CanMove` false))
    (return _output_get_2)
    (else
      (bind _output_get_3 (set `self.CanMove` true))
      (return _output_get_3))))

(fn `RotateTurret`
  (set `self.TurretRotation` (`KismetMathLibrary.RInterpTo_Constant` (`self.TurretRotation`) (`self.AimRotation`) (`GameplayStatics.GetWorldDeltaSeconds`) (`self.TurretTurnSpeed`))))

(fn `UserConstructionScript`)