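; Game mode for a two-player local multiplayer tank match with a shared camera, scoring and respawns.
; On BeginPlay it recreates the local players, spawns the camera and HUD, then spawns a tank at each spawn point for its matching controller to possess.
; Tank destruction events remove the victim from the camera and credit the killer through ACPlayerScores.
; That score either ends the game or the victim's index-matched spawn point respawns it.
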(event `self.ReceiveBeginPlay`
  (`self.RemovePlayers`)
  (`self.SetUpPlayers` 2)
  (bind _outactors (`GameplayStatics.GetAllActorsOfClass` "/Game/TankProject/BP_SpawnPoint.BP_SpawnPoint_C"))
  (set `self.SpawnPoints` _outactors)
  (bind _returnvalue (`|SpawnActorFromClass` "/Game/TankProject/BP_Camera.BP_Camera_C" (`KismetMathLibrary.MakeTransform` (0.0 0.0 0.0)) "Undefined" "MultiplyWithRoot" null null))
  (set `self.CameraActor` _returnvalue)
  (bind _returnvalue_2 (`|CreateWidget` "/Game/TankProject/UI/W_GameHUD.W_GameHUD_C"))
  (set `self.GameHUD` _returnvalue_2)
  (for (_ _array_index) (`self.SpawnPoints`)
    (`self.SpawnTank` _array_index))
  (`/Game/TankProject/BP_Camera.Init` (`self.CameraActor`))
  (`UserWidget.AddToViewport` (`self.GameHUD`) 0)
  (for _array_element (`self.PlayerList`)
    (set `/Game/TankProject/Tank/BP_Tank_Base.CanReceiveInput` true _array_element)))

(event `TankDestroyed`
  (params (PlayerKilled :type "Controller Object Reference") (KilledBy :type "Controller Object Reference"))
  (bind _returnvalue (`Controller.K2_GetPawn` PlayerKilled))
  (`/Game/TankProject/BP_Camera.RemovePlayer` (`self.CameraActor`) _returnvalue)
  (bind (_canend _scoringplayerid) (`/Game/TankProject/AC_PlayerScores.AddScore` (`self.AC_PlayerScores`) (`/Game/TankProject/Tank/BP_Tank_Base.TankID` (cast `/Game/TankProject/Tank/BP_Tank_Base` (`Controller.K2_GetPawn` KilledBy) :!pure true)) 1))
  (if _canend
    (`self.GameEnd` _scoringplayerid)
    (`KismetSystemLibrary.PrintString` "GameEnd")
    (else
      (`/Game/TankProject/BP_SpawnPoint.RespawnTank` (`|GetArrayItem` (`self.SpawnPoints`) (`KismetArrayLibrary.Array_Find` (`self.PlayerList`) (cast `/Game/TankProject/Tank/BP_Tank_Base` _returnvalue :!pure true))) _returnvalue))))

(fn `RemovePlayers`
  (for _index (range (`GameplayStatics.GetNumLocalPlayerControllers`))
    (`GameplayStatics.RemovePlayer` (`GameplayStatics.GetPlayerControllerFromID` _index) true))
  (return))

(fn `SetUpPlayers`
  (params (NumberOfPlayers :type Integer :default 1))
  (for _index (range NumberOfPlayers)
    (bind _returnvalue (`GameplayStatics.CreatePlayer` _index))
    (`KismetArrayLibrary.Array_AddUnique` (`self.PlayerControllerList`) _returnvalue))
  (return))

(fn `SpawnTank`
  (params (TankID :type Integer))
  (bind _returnvalue (`GameplayStatics.GetPlayerController` TankID))
  (bind _returnvalue_2 (`|SpawnActorFromClass` "/Game/TankProject/Tank/BP_Tank_Base.BP_Tank_Base_C" (`self.GetTransform` (`|GetArrayItem` (`self.SpawnPoints`) TankID)) "AdjustIfPossibleButAlwaysSpawn" "MultiplyWithRoot" null TankID null))
  (`KismetArrayLibrary.Array_AddUnique` (`self.PlayerList`) _returnvalue_2)
  (`/Game/TankProject/BP_Camera.AddPlayer` (`self.CameraActor`) _returnvalue_2)
  (add `/Game/TankProject/Tank/BP_Tank_Base.TankDestroyed` _returnvalue_2 (`|CreateDelegate` :!event `TankDestroyed`))
  (`/Engine/EditorBlueprintResources/StandardMacros.IsValid` _returnvalue
    (:`Is Valid`
      (`Controller.Possess` _returnvalue _returnvalue_2)
      (return))
    (:`Is Not Valid`
      (return))))

(fn `UserConstructionScript`)