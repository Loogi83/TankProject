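; BP_SpawnPoint is a spawn point that respawns a tank at its transform after a delay.
; RespawnTank stores the tank and starts a timer, pausing while something overlaps the Box and resuming on any end overlap.
; When it fires, it teleports the tank, adds it to the GM_Tank camera actor, re-enables its player input and clears the reference.
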(event `self.ReceiveBeginPlay`
  (bind _asgm_tank (cast `/Game/TankProject/GM_Tank` (`GameplayStatics.GetGameMode`)))
  (set `self.As GM Tank` _asgm_tank))

(event `RespawnTank`
  (params (TankToRespawn :type "Pawn Object Reference"))
  (set `self.Tank to Respawn` TankToRespawn)
  (bind _returnvalue (`KismetSystemLibrary.K2_SetTimerDelegate` (delegate `Respawn`) (`self.RespawnDelay`)))
  (set `self.RespawnHandle` _returnvalue))

(event `Respawn`
  (bind _tank_to_respawn (`self.Tank to Respawn`))
  (`self.K2_SetActorTransform` (`self.Tank to Respawn`) (`self.GetTransform`) false true)
  (`/Game/TankProject/BP_Camera.AddPlayer` (`/Game/TankProject/GM_Tank.CameraActor` (`self.As GM Tank`)) _tank_to_respawn)
  (bind _asplayer_controller (cast `PlayerController` (`Pawn.GetController` _tank_to_respawn)))
  (`self.EnableInput` (`self.Tank to Respawn`) _asplayer_controller)
  (set `self.Tank to Respawn` null))

(event `self.Box.OnComponentBeginOverlap`
  (params (OverlappedComponent :type "PrimitiveComponent Object Reference") (OtherActor :type "Actor Object Reference") (OtherComp :type "PrimitiveComponent Object Reference") (OtherBodyIndex :type Integer) (bFromSweep :type Boolean) (SweepResult :type "HitResult Structure (by ref)"))
  (`KismetSystemLibrary.K2_PauseTimerHandle` (`self.RespawnHandle`)))

(event `self.Box.OnComponentEndOverlap`
  (params (OverlappedComponent :type "PrimitiveComponent Object Reference") (OtherActor :type "Actor Object Reference") (OtherComp :type "PrimitiveComponent Object Reference") (OtherBodyIndex :type Integer))
  (`KismetSystemLibrary.K2_UnPauseTimerHandle` (`self.RespawnHandle`)))

(fn `UserConstructionScript`)