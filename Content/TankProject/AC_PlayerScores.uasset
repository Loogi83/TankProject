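; AC_PlayerScores is an actor component on the GM_Tank game mode that tracks each player's score in the tank game.
; BeginPlay caches the owning GM_Tank.
; AddScore adds points to the player's entry in a score map keyed by player ID and pushes the new total to the game mode's HUD.
; It returns the scoring player's ID and whether that total has reached MaxScore, signalling that the game can end.
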(event `self.ReceiveBeginPlay`
  (bind _asgm_tank (cast `/Game/TankProject/GM_Tank` (`self.GetOwner`)))
  (set `self.As GM Tank` _asgm_tank))

(fn `AddScore`
  (params (PlayerID :type Integer) (ScoreToAdd :type Integer))
  (returns (CanEnd :type Boolean) (ScoringPlayerID :type Integer))
  (bind _value (`BlueprintMapLibrary.Map_Find` (`self.PlayerScores`) (`local.PlayerID`)))
  (`BlueprintMapLibrary.Map_Add` (`self.PlayerScores`) PlayerID (+ ScoreToAdd _value))
  (`/Game/TankProject/UI/W_GameHUD.UpdateScore` (`/Game/TankProject/GM_Tank.GameHUD` (`self.As GM Tank`)) (`local.PlayerID`) _value)
  (return (>= _value (`self.MaxScore`)) (`local.PlayerID`)))